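; BP_SoundArea is a box volume that scatters random one-shot sounds inside itself while something overlaps it.
; Begin overlap starts a Delay-driven loop that rolls SoundChance each pass and, on success, plays Sound at a random point within the box.
; End overlap sets Done, which is checked before each delay, so one more roll can follow exit.
; Overlaps are not filtered by actor, and a FadeOut node is left unconnected.
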(event `self.Box.OnComponentBeginOverlap`
  (params (OverlappedComponent :type "PrimitiveComponent Object Reference") (OtherActor :type "Actor Object Reference") (OtherComp :type "PrimitiveComponent Object Reference") (OtherBodyIndex :type Integer) (bFromSweep :type Boolean) (SweepResult :type "HitResult Structure (by ref)"))
  (bind _box (`self.Box`))
  (set `self.Done` false)
  (if (`KismetMathLibrary.RandomBoolWithWeight` (`self.Sound Chance`)) :!label _label
    (`GameplayStatics.PlaySoundAtLocation` (`self.Sound`) (`KismetMathLibrary.RandomPointInBoundingBox` (`SceneComponent.K2_GetComponentLocation` _box) (`BoxComponent.GetScaledBoxExtent` _box)) (struct) 1.0 1.0 0.0 null null null))
  (if (not (`self.Done`))
    (`KismetSystemLibrary.Delay` (`self.Delay Duration`))
    (goto _label)))

(event `self.Box.OnComponentEndOverlap`
  (params (OverlappedComponent :type "PrimitiveComponent Object Reference") (OtherActor :type "Actor Object Reference") (OtherComp :type "PrimitiveComponent Object Reference") (OtherBodyIndex :type Integer))
  (set `self.Done` true))

(fn `UserConstructionScript`)
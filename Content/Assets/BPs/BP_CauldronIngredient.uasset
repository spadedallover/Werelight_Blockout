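; BP_CauldronIngredient is a collectible cauldron ingredient that the player picks up by interacting with it.
; Interactwith increments NumberofObjects on the FirstPersonCharacter, destroys the actor, then adds a CauldronIngredients_Widget to the viewport.
; A one-second Delay before RemoveAllWidgets follows DestroyActor, so that cleanup is unlikely to run.
; The PickUpBox overlap event is empty, and CheckInventory is a stub that returns false.
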(event `/Game/Assets/BPs/BP_LightInterface.InteractWith`
  (params (InteractWith :type "Vector Structure"))
  (bind _asfirst_person_character (cast `/Game/FirstPersonBP/Blueprints/FirstPersonCharacter` (`GameplayStatics.GetPlayerPawn` 0)))
  (set `/Game/FirstPersonBP/Blueprints/FirstPersonCharacter.NumberofObjects` (+ (`/Game/FirstPersonBP/Blueprints/FirstPersonCharacter.NumberofObjects` _asfirst_person_character) 1) _asfirst_person_character)
  (`self.K2_DestroyActor`)
  (bind _returnvalue (`|CreateWidget` "/Game/Assets/BPs/CauldronIngredients_Widget.CauldronIngredients_Widget_C"))
  (bind _output_get (set `self.ingredients_Widget` _returnvalue))
  (`UserWidget.AddToViewport` _output_get 0)
  (`KismetSystemLibrary.Delay` 1.0)
  (`WidgetLayoutLibrary.RemoveAllWidgets`))

(event `self.PickUpBox.OnComponentBeginOverlap`
  (params (OverlappedComponent :type "PrimitiveComponent Object Reference") (OtherActor :type "Actor Object Reference") (OtherComp :type "PrimitiveComponent Object Reference") (OtherBodyIndex :type Integer) (bFromSweep :type Boolean) (SweepResult :type "HitResult Structure (by ref)")))

(fn `CheckInventory`
  (params (Item :type String))
  (returns (PickedUp :type Boolean))
  (return false))

(fn `UserConstructionScript`)
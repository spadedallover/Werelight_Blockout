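; Time-scrubbing actor that lets the player run a Level Sequence forward or backward while inside its box trigger.
; The box toggles input; holding E or Q plays or reverses the sequence, stopping at either end unless it is looped, and release pauses it.
; While scrubbing, a bell chime repeats and global audio pitch shifts.
; Tick maps sequence time to grass opacity through a Material Parameter Collection.
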(event `self.ReceiveBeginPlay`
  ;[1 1 1] Scrub Time/Set Play Rate/Set Grass Opacity
  (`MovieSceneSequencePlayer.JumpToFrame` (`LevelSequenceActor.SequencePlayer` (`self.LevelSequence`)) (make `FrameTime` (make `FrameNumber` (`self.Start Frame`))))
  (`MovieSceneSequencePlayer.SetPlayRate` (`LevelSequenceActor.SequencePlayer` (`self.LevelSequence`)) (`self.PlayRate`))
  (`KismetMaterialLibrary.SetScalarParameterValue` "/Game/Assets/Materials/MPC_GrassParamCollec.MPC_GrassParamCollec" "Grass Opacity"))

(event `self.Box.OnComponentEndOverlap`
  (params (OverlappedComponent :type "PrimitiveComponent Object Reference") (OtherActor :type "Actor Object Reference") (OtherComp :type "PrimitiveComponent Object Reference") (OtherBodyIndex :type Integer))
  ;[1 1 1] Overlap Events
  (set `self.CanGrassGrow?` false)
  (`self.DisableInput` (`GameplayStatics.GetPlayerController` 0))
  (`MovieSceneSequencePlayer.Pause` (`LevelSequenceActor.SequencePlayer` (`self.LevelSequence`))))

(event `self.ReceiveTick`
  (params (DeltaSeconds :type "Float (single-precision)"))
  ;[1 1 1] Vertex Colored Grass Growth
  (if (`self.CanGrassGrow?`)
    (`KismetMaterialLibrary.SetScalarParameterValue` "/Game/Assets/Materials/MPC_GrassParamCollec.MPC_GrassParamCollec" "Grass Opacity" (`KismetMathLibrary.Lerp` 0.0 1.0 (`KismetMathLibrary.FClamp` (/ (`TimeManagementBlueprintLibrary.Conv_QualifiedFrameTimeToSeconds` (`MovieSceneSequencePlayer.GetCurrentTime` (`LevelSequenceActor.SequencePlayer` (`self.LevelSequence`)))) 5.0) 0.0 1.15)))))

(event `self.Box.OnComponentBeginOverlap`
  (params (OverlappedComponent :type "PrimitiveComponent Object Reference") (OtherActor :type "Actor Object Reference") (OtherComp :type "PrimitiveComponent Object Reference") (OtherBodyIndex :type Integer) (bFromSweep :type Boolean) (SweepResult :type "HitResult Structure (by ref)"))
  ;[1 1 1] Overlap Events
  (set `self.CanGrassGrow?` true)
  (`self.EnableInput` (`GameplayStatics.GetPlayerController` 0)))

(event `Key|E`
  (params (Key :type "Key Structure"))
  (bind _sequenceplayer (`LevelSequenceActor.SequencePlayer` (`self.LevelSequence`)))
  (bind _sequenceplayer_2 (`LevelSequenceActor.SequencePlayer` (`self.LevelSequence`)))
  (bind _returnvalue (>= (`.Value` (break `FrameNumber` (`KismetMathLibrary.BreakQualifiedFrameTime` (`MovieSceneSequencePlayer.GetCurrentTime` _sequenceplayer)))) (- (`.Value` (break `FrameNumber` (`KismetMathLibrary.BreakQualifiedFrameTime` (`MovieSceneSequencePlayer.GetEndTime` _sequenceplayer)))) 1)))
  ;[1 1 1] Time Mechanic
  (:`Pressed`
    (if (`self.LoopedSequence?`)
      (`MovieSceneSequencePlayer.Play` _sequenceplayer_2 :!label _label)
      ;[1 1 1] Audio
      (if (or _returnvalue (`MovieSceneSequencePlayer.IsPaused` _sequenceplayer_2)) :!label _label_2
        _
        (else
          (`GameplayStatics.SetGlobalPitchModulation` -10.0 100.0)
          (`GameplayStatics.PlaySoundAtLocation` "/Game/Assets/Sounds/BellChime1.BellChime1" (`self.K2_GetActorLocation` (`GameplayStatics.GetPlayerCharacter` 0)) (struct) 1.0 1.0 0.0 null null null)
          (`KismetSystemLibrary.Delay` 0.5)
          (goto _label_2)))
      (elif _returnvalue
        (`MovieSceneSequencePlayer.Pause` _sequenceplayer_2 :!label _label_3)
        (else
          (goto _label))))
    (`GameplayStatics.SetGlobalPitchModulation` 1.0 10.0 :!label _label_4))
  (:`Released`
    (goto _label_3)))

(event `Key|Q`
  (params (Key :type "Key Structure"))
  (bind _sequenceplayer (`LevelSequenceActor.SequencePlayer` (`self.LevelSequence`)))
  (bind _sequenceplayer_2 (`LevelSequenceActor.SequencePlayer` (`self.LevelSequence`)))
  (bind _returnvalue (<= (`.Value` (break `FrameNumber` (`KismetMathLibrary.BreakQualifiedFrameTime` (`MovieSceneSequencePlayer.GetCurrentTime` _sequenceplayer)))) (`.Value` (break `FrameNumber` (`KismetMathLibrary.BreakQualifiedFrameTime` (`MovieSceneSequencePlayer.GetStartTime` _sequenceplayer))))))
  ;[1 1 1] Time Mechanic
  (:`Pressed`
    (if (`self.LoopedSequence?`)
      _
      (elif _returnvalue
        (goto _label_3)
        (else
          _)))
    (`MovieSceneSequencePlayer.PlayReverse` _sequenceplayer_2)
    ;[1 1 1] Audio
    (if (or (`MovieSceneSequencePlayer.IsPaused` _sequenceplayer_2) _returnvalue) :!label _label_5
      (goto _label_4)
      (else
        (`GameplayStatics.SetGlobalPitchModulation` 10.0 100.0)
        (`GameplayStatics.PlaySoundAtLocation` "/Game/Assets/Sounds/BellChime1.BellChime1" (`self.K2_GetActorLocation` (`GameplayStatics.GetPlayerCharacter` 0)) (struct) 1.0 1.0 0.0 null null null)
        (`KismetSystemLibrary.Delay` 0.5)
        (goto _label_5))))
  (:`Released`
    (goto _label_3)))

(fn `UserConstructionScript`)
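; Floating island actor that spins its Box a fixed yaw step every tick and moves it along a timeline.
; The timeline, scaled by Speed, drives offsets up to Distance horizontally (X or Y) and/or vertically, per boolean flags.
; BeginPlay snaps Bricks to a random quarter-turn yaw.
; The construction script sets a stream-seeded starting island yaw and positions start/end arrows to mark the travel range.
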(event `self.ReceiveTick`
  (params (DeltaSeconds :type "Float (single-precision)"))
  ;[1 1 1] Constant Rotation
  (`SceneComponent.K2_AddRelativeRotation` (`self.Box`) (`KismetMathLibrary.MakeRotator` 0.0 0.0 (`self.Rotation Amount`)) false false))

(event `self.ReceiveBeginPlay`
  (bind _x_axis_ (`self.X Axis?`))
  ;[1 1 1] Movement
  (`|ExecutionSequence`
    (:`then_0`
      (`TimelineComponent.SetPlayRate` (`self.Timeline_0`) (`self.Speed`))
      (bind (_direction _newtrack_0) (`Timeline|Timeline_0`)
        (:`Update`
          (bind _returnvalue (`KismetMathLibrary.Lerp` 0.0 (`self.Distance`) _newtrack_0))
          (bind _returnvalue_2 (select `bool` (`self.LeftRight?`) :`true` _returnvalue))
          (`SceneComponent.K2_SetRelativeLocation` (`self.Box`) (`KismetMathLibrary.MakeVector` (select `bool` _x_axis_ :`true` _returnvalue_2) (select `bool` _x_axis_ :`false` _returnvalue_2) (select `bool` (`self.UpDown?`) :`true` _returnvalue)) false false))))
    (:`then_1`
      ;[1 1 1] Random Brick Rotation x 90
      (`SceneComponent.K2_SetRelativeRotation` (`self.Bricks`) (`KismetMathLibrary.MakeRotator` 0.0 0.0 (select `int` (`KismetMathLibrary.RandomIntegerInRange` 0 3) :`0` 0.0 :`1` 90.0 :`2` 180.0 :`3` 270.0 :!type "Float (single-precision)")) false false))))

(fn `UserConstructionScript`
  (bind _leftright_ (`self.LeftRight?`))
  (bind _leftright__2 (`self.LeftRight?`))
  (bind _returnvalue (+ (`self.Distance`) 50.0))
  (bind _returnvalue_2 (+ (* -1 (`self.Distance`)) -50.0))
  (`SceneComponent.K2_SetRelativeRotation` (`self.Box`) (`KismetMathLibrary.MakeRotator` 0.0 0.0 (`KismetMathLibrary.RandomFloatInRangeFromStream` 0.0 360.0 (`self.Random Island Rotation`))) false false)
  (`SceneComponent.K2_SetRelativeLocation` (`self.ArrowEnd`) (`KismetMathLibrary.MakeVector` (select `bool` _leftright_ :`false` (`self.ArrowDistance`) :`true` _returnvalue) 0.0 (select `bool` _leftright_ :`false` _returnvalue :`true` 350.0)) false false)
  (`SceneComponent.K2_SetRelativeLocation` (`self.ArrowStart`) (`KismetMathLibrary.MakeVector` (select `bool` _leftright__2 :`false` (`self.ArrowDistance`) :`true` _returnvalue_2) 0.0 (select `bool` _leftright__2 :`false` _returnvalue_2 :`true` 350.0)) false false)
  (`SceneComponent.K2_SetRelativeRotation` (`self.ArrowStart`) (`KismetMathLibrary.MakeRotator` 0.0 (select `bool` (`self.LeftRight?`) :`false` 180.0 :`true` -90.0 :!type "Float (single-precision)")) false false)
  (`SceneComponent.K2_SetRelativeRotation` (`self.ArrowEnd`) (`KismetMathLibrary.MakeRotator` 0.0 (select `bool` (`self.LeftRight?`) :`false` 180.0 :`true` -90.0 :!type "Float (single-precision)")) false false))
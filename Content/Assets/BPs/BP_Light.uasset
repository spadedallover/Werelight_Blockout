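; BP_Light is a light actor that signals a memory unlock when switched.
; SwitchLight casts the player to FirstPersonCharacter, then toggles visibility of the point light, Werelight and smoke, and plays a temple bell at world origin.
; It shows MemoryUnlock_Widget, then after a delay removes all widgets, not just its own.
; LightFunction, GetPassedThroughDoorNumber and CheckInventory are stubs, and the door-counter and broadcast nodes are disconnected.
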(event `/Game/Assets/BPs/BP_LightInterface.LightFunction`
  (params (LightFunction :type "Actor Object Reference")))

(event `SwitchLight`
  (cast `/Game/FirstPersonBP/Blueprints/FirstPersonCharacter` (`GameplayStatics.GetPlayerCharacter` 0))
  (if true
    (`SceneComponent.ToggleVisibility` (`self.PointLight`) false)
    (`SceneComponent.ToggleVisibility` (`self.Werelight`) false)
    (`SceneComponent.ToggleVisibility` (`self.P_Smoke`) false)
    (`GameplayStatics.PlaySoundAtLocation` "/Game/Assets/Sounds/Temple_Bell-SoundBible_com-756181215.Temple_Bell-SoundBible_com-756181215" (0.0 0.0 0.0) (struct) 1.0 1.0 0.0 null null null)
    (bind _returnvalue (`|CreateWidget` "/Game/Assets/BPs/UI/MemoryUnlock_Widget.MemoryUnlock_Widget_C"))
    (bind _output_get (set `self.Widget` _returnvalue))
    (`UserWidget.AddToViewport` _output_get 0)
    (`KismetSystemLibrary.Delay` 3.0)
    (`WidgetLayoutLibrary.RemoveAllWidgets`)))

(fn `CheckInventory`
  (params (Item :type String))
  (returns (PickedUp :type Boolean))
  (return false))

(fn `GetPassedThroughDoorNumber`
  (returns (NumberofTimesDoorHassBeenPassedThrough :type Integer))
  (return 0))

(fn `UserConstructionScript`)
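; BP_EndGame is an end-of-game trigger that plays the closing sequence when its Box component is overlapped.
; The overlap shows a fade-to-black widget, then the UI_Credits widget, then opens the MainMenu level.
; Each step waits with a Delay set to the end time of that widget's animation, so timing follows animation length.
; The overlap has no check on which actor entered or whether it already fired.
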(event `self.Box.OnComponentBeginOverlap`
  (params (OverlappedComponent :type "PrimitiveComponent Object Reference") (OtherActor :type "Actor Object Reference") (OtherComp :type "PrimitiveComponent Object Reference") (OtherBodyIndex :type Integer) (bFromSweep :type Boolean) (SweepResult :type "HitResult Structure (by ref)"))
  ;[1 1 1] Fade Out
  (bind _returnvalue (`|CreateWidget` "/Game/Assets/BPs/UI/UI_FadeToBlack.UI_FadeToBlack_C"))
  (`UserWidget.AddToViewport` _returnvalue 0)
  (`KismetSystemLibrary.Delay` (`WidgetAnimation.GetEndTime` (`/Game/Assets/BPs/UI/UI_FadeToBlack.NewAnimation` _returnvalue)))
  ;[1 1 1] Credits
  (bind _returnvalue_2 (`|CreateWidget` "/Game/Assets/BPs/UI/UI_Credits.UI_Credits_C"))
  (`UserWidget.AddToViewport` _returnvalue_2 0)
  (`KismetSystemLibrary.Delay` (`WidgetAnimation.GetEndTime` (`/Game/Assets/BPs/UI/UI_Credits.SCROLLING` _returnvalue_2)))
  ;[1 1 1] Main Menu
  (`GameplayStatics.OpenLevel` "MainMenu"))

(fn `UserConstructionScript`)
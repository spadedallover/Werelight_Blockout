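; BP_NemerleDialogue is a trigger that shows a three-part Nemerle dialogue on screen when its Box component is overlapped.
; On overlap it creates the A, B and C dialogue widgets in turn, showing each for a fixed delay before removing it.
; A DoOnce blocks retriggering during the sequence and resets at the end, so the dialogue can play again.
; The overlapping actor is not filtered.
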(event `self.Box.OnComponentBeginOverlap`
  (params (OverlappedComponent :type "PrimitiveComponent Object Reference") (OtherActor :type "Actor Object Reference") (OtherComp :type "PrimitiveComponent Object Reference") (OtherBodyIndex :type Integer) (bFromSweep :type Boolean) (SweepResult :type "HitResult Structure (by ref)"))
  (`/Engine/EditorBlueprintResources/StandardMacros.DoOnce` false :!label _label
    (:`Completed`
      (bind _returnvalue (`|CreateWidget` "/Game/Assets/BPs/UI/UI_NemDialogueA.UI_NemDialogueA_C"))
      (`UserWidget.AddToViewport` _returnvalue 0)
      (`KismetSystemLibrary.Delay` 3.0)
      (`Widget.RemoveFromParent` _returnvalue)
      (bind _returnvalue_2 (`|CreateWidget` "/Game/Assets/BPs/UI/UI_NemDialogueb.UI_NemDialogueB_C"))
      (`UserWidget.AddToViewport` _returnvalue_2 0)
      (`KismetSystemLibrary.Delay` 3.0)
      (`Widget.RemoveFromParent` _returnvalue_2)
      (bind _returnvalue_3 (`|CreateWidget` "/Game/Assets/BPs/UI/UI_NemDialogueC.UI_NemDialogueC_C"))
      (`UserWidget.AddToViewport` _returnvalue_3 0)
      (`KismetSystemLibrary.Delay` 3.0)
      (`Widget.RemoveFromParent` _returnvalue_3)
      (goto _label :!via `Reset`))))

(fn `UserConstructionScript`)
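; Banner actor that sets the static mesh of its Banner component from an array of banner meshes.
; The construction script uses either a random index from 0 to 3, when RandomIndex is set, or the chosen BannerIndex.
; The random pick uses a hard-coded range and no seed, so it can change whenever construction reruns.
; The event graph holds only disabled placeholder events, so there is no gameplay logic.
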(fn `UserConstructionScript`
  (bind _banner (`self.Banner`))
  (if (`self.Random Index?`)
    (`StaticMeshComponent.SetStaticMesh` _banner (`|GetArrayItem` (`self.BannerArray`) (`KismetMathLibrary.RandomIntegerInRange` 0 3)))
    (else
      (`StaticMeshComponent.SetStaticMesh` _banner (`|GetArrayItem` (`self.BannerArray`) (`self.BannerIndex`))))))
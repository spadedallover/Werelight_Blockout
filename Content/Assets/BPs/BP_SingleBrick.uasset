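; BP_SingleBrick is a brick actor whose mesh moves along local Z, within a 100-unit range, in a repeating animation.
; The construction script picks a random static mesh from the NewMesh array.
; On BeginPlay a timeline starts at a random position and drives the mesh's relative location through a lerp.
; Each time it finishes, it restarts with a randomized play rate, so separate instances move out of sync.
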(event `self.ReceiveBeginPlay`
  (`TimelineComponent.SetPlaybackPosition` (`self.Timeline_0`) (`KismetMathLibrary.RandomFloatInRange` 0.0 2.9) false true)
  (bind (_direction _newtrack_0) (`Timeline|Timeline_0` :!label _label)
    (:`Update`
      (`SceneComponent.K2_SetRelativeLocation` (`self.StaticMesh`) (`KismetMathLibrary.VLerp` (0.0 0.0 0.0) (0.0 0.0 100.0) _newtrack_0) false false))
    (:`Finished`
      (`TimelineComponent.SetPlayRate` (`self.Timeline_0`) (`KismetMathLibrary.RandomFloatInRange` 0.75 1.25))
      (goto _label :!via `PlayFromStart`))))

(fn `UserConstructionScript`
  (bind _new_mesh (`self.New Mesh`))
  (`StaticMeshComponent.SetStaticMesh` (`self.StaticMesh`) (`|GetArrayItem` _new_mesh (`KismetMathLibrary.RandomIntegerInRange` 0 (- (`KismetArrayLibrary.Array_Length` _new_mesh) 1)))))
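; Manager actor for a linked pair of portals, meant to drive their scene captures from the player's camera view.
; Each update function places the opposite portal's PortalCapture at the camera location offset by the translation between portals, copying camera rotation without compensating for portal orientation.
; BeginPlay only caches the FirstPersonCharacter.
; The update chain, gated on CanOpenDoor, is disconnected from the empty Tick, so captures never move.
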(event `self.ReceiveBeginPlay`
  (bind _asfirst_person_character (cast `/Game/FirstPersonBP/Blueprints/FirstPersonCharacter` (`GameplayStatics.GetPlayerCharacter` 0))))

(event `self.ReceiveTick`
  (params (DeltaSeconds :type "Float (single-precision)")))

(fn `UpdatePortal1`
  (bind _portal2 (`self.Portal2`))
  (bind _transformcomponent (`PlayerCameraManager.TransformComponent` (`GameplayStatics.GetPlayerCameraManager` 0)))
  (`SceneComponent.K2_SetWorldLocationAndRotation` (`/Game/Assets/BPs/BP_Portal2.portalCapture` _portal2) (+ (- (`SceneComponent.K2_GetComponentLocation` (`/Game/Assets/BPs/BP_Portal2.DefaultSceneRoot` _portal2)) (`SceneComponent.K2_GetComponentLocation` (`/Game/Assets/BPs/BP_Portal1.DefaultSceneRoot` (`self.Portal1`)))) (`SceneComponent.K2_GetComponentLocation` _transformcomponent)) (`SceneComponent.K2_GetComponentRotation` _transformcomponent) false false))

(fn `UpdatePortal2`
  (bind _portal1 (`self.Portal1`))
  (bind _transformcomponent (`PlayerCameraManager.TransformComponent` (`GameplayStatics.GetPlayerCameraManager` 0)))
  (`SceneComponent.K2_SetWorldLocationAndRotation` (`/Game/Assets/BPs/BP_Portal1.portalCapture` _portal1) (+ (- (`SceneComponent.K2_GetComponentLocation` (`/Game/Assets/BPs/BP_Portal1.DefaultSceneRoot` _portal1)) (`SceneComponent.K2_GetComponentLocation` (`/Game/Assets/BPs/BP_Portal2.DefaultSceneRoot` (`self.Portal2`)))) (`SceneComponent.K2_GetComponentLocation` _transformcomponent)) (`SceneComponent.K2_GetComponentRotation` _transformcomponent) false false))

(fn `UserConstructionScript`)
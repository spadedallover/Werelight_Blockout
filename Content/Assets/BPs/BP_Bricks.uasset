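; BP_Bricks is a spawner actor that scatters BP_SingleBrick actors at random points inside a bounding box on BeginPlay.
; It passes its rotation, max height and playback time settings to each of the spawned bricks.
; The construction script sizes the box from a uniform or per-axis extent and scales the arrow group by that size or the average extent.
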(event `self.ReceiveBeginPlay`
  ;[1 1 1] Set Brick Spawn Amount
  (for _ (range (`self.Brick Amount`))
    ;[1 1 1] Spawn Brick in Bounding Box
    (`|SpawnActorFromClass` "/Game/Assets/BPs/BP_SingleBrick.BP_SingleBrick_C" (`KismetMathLibrary.Conv_VectorToTransform` (`KismetMathLibrary.RandomPointInBoundingBox` (`SceneComponent.K2_GetComponentLocation` (`self.boundingBox`)) (select `bool` (`self.Uniform Box Extent?`) :`false` (`self.Box Extent`) :`true` (`KismetMathLibrary.Conv_DoubleToVector` (`self.Box Extent Size`))))) "Undefined" "OverrideRootScale" null (`self.Add Rotation Amount`) (`self.Max Set Rotation`) (`self.X Rotation`) (`self.Y Rotation`) (`self.Z Rotation`) (`self.Max Height`) (`self.Max Playback Time`) (`self.Min Playback Time`) null)))

(fn `UserConstructionScript`
  (bind (_box_extent_x _box_extent_y _box_extent_z) (`KismetMathLibrary.BreakVector` (`self.Box Extent`)))
  (bind _arrowscalegroup (`self.ArrowScaleGroup`))
  (bind _arrowscalegroup_2 (`self.ArrowScaleGroup`))
  (bind _box_extent_size (`self.Box Extent Size`))
  (if (`self.Uniform Box Extent?`)
    ;[1 1 1] Arrow Resize
    (`SceneComponent.SetWorldScale3D` _arrowscalegroup_2 (* (`SceneComponent.K2_GetComponentScale` _arrowscalegroup_2) (/ (`self.Box Extent Size`) 175.0)))
    (`BoxComponent.SetBoxExtent` (`self.boundingBox`) (`KismetMathLibrary.MakeVector` _box_extent_size _box_extent_size _box_extent_size) true)
    (else
      ;[1 1 1] Arrow Resize
      (`SceneComponent.SetWorldScale3D` _arrowscalegroup (* (`SceneComponent.K2_GetComponentScale` _arrowscalegroup) (/ (/ (+ (+ _box_extent_x _box_extent_y) _box_extent_z) 3.0) 175.0)))
      (`BoxComponent.SetBoxExtent` (`self.boundingBox`) (`self.Box Extent`) true))))
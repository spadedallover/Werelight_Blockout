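; BP_TableSpline is a construction-script actor that tiles static meshes, presumably table pieces, along an editable spline.
; It adds one collidable spline mesh per SectionLength step, taking local positions and length-clamped tangents from the spline.
; Each segment picks a random mesh from the Mesh array and continues an accumulating roll, whose step scales with RollAmount and the spline's point count.
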(fn `UserConstructionScript`
  (bind _currentroll (`self.CurrentRoll`))
  (bind _spline (`self.Spline`))
  (bind _sectionlength (`self.SectionLength`))
  (bind _sectionlength_2 (`self.SectionLength`))
  (bind _mesh (`self.mesh`))
  (for _index (range (+ (`KismetMathLibrary.FTrunc` (/ (`SplineComponent.GetSplineLength` (`self.Spline`)) (`self.SectionLength`))) 1))
    (bind _returnvalue (`AddComponent|NODE_AddSplineMeshComponent-0`))
    (`SplineMeshComponent.SetStartRoll` _returnvalue _currentroll true)
    (bind _output_get (set `self.CurrentRoll` (+ _currentroll (* (`KismetMathLibrary.Conv_IntToDouble` (- (`SplineComponent.GetNumberOfSplinePoints` (`self.Spline`)) 1)) (`self.RollAmount`)))))
    (`SplineMeshComponent.SetEndRoll` _returnvalue _output_get true)
    (`PrimitiveComponent.SetCollisionEnabled` _returnvalue "QueryAndPhysics")
    (`SplineMeshComponent.SetForwardAxis` _returnvalue (`self.Forward Axis`) true)
    (bind _returnvalue_2 (* _index _sectionlength))
    (bind _returnvalue_3 (* (+ _index 1) _sectionlength))
    (`SplineMeshComponent.SetStartAndEnd` _returnvalue (`SplineComponent.GetLocationAtDistanceAlongSpline` _spline _returnvalue_2 "Local") (`KismetMathLibrary.ClampVectorSize` (`SplineComponent.GetTangentAtDistanceAlongSpline` _spline _returnvalue_2 "Local") 0.0 _sectionlength_2) (`SplineComponent.GetLocationAtDistanceAlongSpline` _spline _returnvalue_3 "Local") (`KismetMathLibrary.ClampVectorSize` (`SplineComponent.GetTangentAtDistanceAlongSpline` _spline _returnvalue_3 "Local") 0.0 _sectionlength_2) true)
    (`StaticMeshComponent.SetStaticMesh` _returnvalue (`|GetArrayItem` _mesh (`KismetMathLibrary.RandomIntegerInRange` 0 (- (`KismetArrayLibrary.Array_Length` _mesh) 1))))))
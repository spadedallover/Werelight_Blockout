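; BP_LightTrigger is a one-shot trigger that switches the level's lights and activates key triggers.
; The first actor overlap, with no filter on the overlapping actor, passes a DoOnce and calls SwitchLight on every BP_Light, then TurnOnTrigger on every BP_TriggerSetKey, both found by class lookup.
; The Trigger component's overlap events are empty, CheckInventory always returns false, and leftover interface-message and player-cast nodes never run.
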(event `self.ReceiveActorBeginOverlap`
  (params (OtherActor :type "Actor Object Reference"))
  (`/Engine/EditorBlueprintResources/StandardMacros.DoOnce` false
    (:`Completed`
      (bind _outactors (`GameplayStatics.GetAllActorsOfClass` "/Game/Assets/BPs/BP_Light.BP_Light_C"))
      (`/Game/Assets/BPs/BP_Light.SwitchLight` _outactors)
      (bind _outactors_2 (`GameplayStatics.GetAllActorsOfClass` "/Game/Assets/BPs/BP_TriggerSetKey.BP_TriggerSetKey_C"))
      (`/Game/Assets/BPs/BP_TriggerSetKey.TurnOnTrigger` _outactors_2))))

(event `self.Trigger.OnComponentBeginOverlap`
  (params (OverlappedComponent :type "PrimitiveComponent Object Reference") (OtherActor :type "Actor Object Reference") (OtherComp :type "PrimitiveComponent Object Reference") (OtherBodyIndex :type Integer) (bFromSweep :type Boolean) (SweepResult :type "HitResult Structure (by ref)")))

(event `self.Trigger.OnComponentEndOverlap`
  (params (OverlappedComponent :type "PrimitiveComponent Object Reference") (OtherActor :type "Actor Object Reference") (OtherComp :type "PrimitiveComponent Object Reference") (OtherBodyIndex :type Integer)))

(fn `CheckInventory`
  (params (Item :type String))
  (returns (PickedUp :type Boolean))
  (return false))

(fn `UserConstructionScript`)
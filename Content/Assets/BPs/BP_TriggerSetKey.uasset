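; BP_TriggerSetKey is a set-key trigger that fires an interaction and switches off its associated lights.
; TurnOnTrigger opens a gate, letting RiseSetkeyTrigger pass through a DoOnce to call SetTriggerInteraction and toggle visibility on the Lights actors' roots.
; Overlap events and CheckInventory are stubs.
; Box-moving timelines, scene lighting and particle toggling are unwired, with a note that particles or Blueprints failed to work.
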(event `/Game/Assets/BPs/BP_LightInterface.Rise_SetkeyTrigger`
  (`/Engine/EditorBlueprintResources/StandardMacros.Gate` true :!label _label
    (:`Exit`
      (`/Engine/EditorBlueprintResources/StandardMacros.DoOnce` false
        (:`Completed`
          (`self.SetTrigger_Interaction`)
          (for _array_element (`self.Lights`)
            (`SceneComponent.ToggleVisibility` (`Actor.RootComponent` _array_element) false)))))))

(event `TurnOnTrigger`
  (goto _label :!via `Open`))

(event `/Game/Assets/BPs/BP_LightInterface.TriggerOverlap`)

(event `self.ReceiveActorBeginOverlap`
  (params (OtherActor :type "Actor Object Reference")))

(event `self.Box.OnComponentEndOverlap`
  (params (OverlappedComponent :type "PrimitiveComponent Object Reference") (OtherActor :type "Actor Object Reference") (OtherComp :type "PrimitiveComponent Object Reference") (OtherBodyIndex :type Integer)))

(fn `CheckInventory`
  (params (Item :type String))
  (returns (PickedUp :type Boolean))
  (return false))

(fn `UserConstructionScript`)
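; Butterfly actor that flaps two wings and is positioned along a spline path.
; The construction script gives both wing components the same configurable mesh.
; On BeginPlay, the Wings timeline drives mirrored wing pitch and sets the butterfly's world transform on each update from the spline, using the Path timeline's value as normalized distance.
; The Path timeline has no play call wired in this graph.
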(event EventBeginPlay
  (bind _spline (Variables|Default|GetSpline))
  (Utilities|FlowControl|Sequence
    (:then_1
      (bind _leftwing (Timeline|Wings Play)
        (:Update
          (Transformation|SetRelativeRotation (Variables|Default|GetButterflyWingLeft) (Math|Rotator|MakeRotator 0.0 (Math|Float|Lerp -7e+01 7e+01 _leftwing) 9e+01) false false)
          (Transformation|SetRelativeRotation (Variables|Default|GetRight) (Math|Rotator|MakeRotator 0.0 (Math|Float|Lerp 7e+01 -7e+01 _leftwing) 9e+01) false false)
          (Transformation|SetWorldTransform (Variables|Default|GetButterflyA) (Math|Transform|MakeTransform (Spline|GetLocationatDistanceAlongSpline _spline (* (Spline|GetSplineLength _spline) (stale _newtrack_0)) "World") (Spline|GetRotationatDistanceAlongSpline _spline (* (Spline|GetSplineLength _spline) (stale _newtrack_0)) "World") "0.100000,0.100000,0.100000") false false))))))

(fn ConstructionScript
  (bind _mesh (Variables|Default|GetMesh))
  (Components|StaticMesh|SetStaticMesh (Variables|Default|GetRight) _mesh)
  (Components|StaticMesh|SetStaticMesh (Variables|Default|GetButterflyWingLeft) _mesh))
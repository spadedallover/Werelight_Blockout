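; Hittable light actor that toggles its light and smoke effect and announces an unlocked memory on screen.
; Switch_Hitlight casts the player to FirstPersonCharacter, toggles visibility of PointLight, Werelight and PSmoke, then prints the memory message.
; BeginPlay calls CallLightInteraction, which is not defined in this graph.
; SwitchLight, GetPassedThroughDoorNumber and CheckInventory are stubs, and the door-counter logic is disconnected.
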(event `SwitchLight`)

(event `Switch_Hitlight`
  (cast `/Game/FirstPersonBP/Blueprints/FirstPersonCharacter` (`GameplayStatics.GetPlayerCharacter` 0))
  (if true
    (`SceneComponent.ToggleVisibility` (`self.PointLight`) false)
    (`SceneComponent.ToggleVisibility` (`self.Werelight`) false)
    (`SceneComponent.ToggleVisibility` (`self.P_Smoke`) false)
    (`KismetSystemLibrary.PrintString` "New Memory Unlocked!")))

(event `self.ReceiveBeginPlay`
  (`self.LightInteraction`))

(fn `CheckInventory`
  (params (Item :type String))
  (returns (PickedUp :type Boolean))
  (return false))

(fn `GetPassedThroughDoorNumber`
  (returns (NumberofTimesDoorHassBeenPassedThrough :type Integer))
  (return 0))

(fn `UserConstructionScript`)
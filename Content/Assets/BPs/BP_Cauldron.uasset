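; BP_Cauldron is an interactable that brews a potion from ingredients the player has collected.
; Interactwith compares the first-person character's NumberofObjects to the required count and deducts it when sufficient.
; A DoOnce then plays the cauldron animation, fires CauldronPotionMade and closes a Gate, which otherwise shows CauldronWidget for three seconds on failed attempts.
; The deduction precedes the DoOnce, so it can repeat; CheckInventory is a stub returning false.
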(event `/Game/Assets/BPs/BP_LightInterface.InteractWith`
  (params (InteractWith :type "Vector Structure"))
  (bind _requirednumberofingredients (`self.RequiredNumberOfIngredients`))
  (`WidgetLayoutLibrary.RemoveAllWidgets`)
  (bind _asfirst_person_character (cast `/Game/FirstPersonBP/Blueprints/FirstPersonCharacter` (`GameplayStatics.GetPlayerPawn` 0)))
  (bind _numberofobjects (`/Game/FirstPersonBP/Blueprints/FirstPersonCharacter.NumberofObjects` _asfirst_person_character))
  (if (>= _numberofobjects _requirednumberofingredients)
    (set `/Game/FirstPersonBP/Blueprints/FirstPersonCharacter.NumberofObjects` (- _numberofobjects _requirednumberofingredients) _asfirst_person_character)
    (`/Engine/EditorBlueprintResources/StandardMacros.DoOnce` false
      (:`Completed`
        (`SkeletalMeshComponent.PlayAnimation` (`self.ChestAnim`) "/Game/Assets/Anim/CauldronAnim_Anim.CauldronAnim_Anim" false)
        (`self.CauldronPotionMade`)
        (goto _label :!via `Close`)))
    (else
      (`/Engine/EditorBlueprintResources/StandardMacros.Gate` false :!label _label
        (:`Exit`
          (bind _returnvalue (`|CreateWidget` "/Game/Assets/BPs/CauldronWidget.CauldronWidget_C"))
          (bind _output_get (set `self.NewVar_0` _returnvalue))
          (`UserWidget.AddToViewport` _output_get 0)
          (`KismetSystemLibrary.Delay` 3.0)
          (`WidgetLayoutLibrary.RemoveAllWidgets`))))))

(event `self.PickupCheckTrigger.OnComponentBeginOverlap`
  (params (OverlappedComponent :type "PrimitiveComponent Object Reference") (OtherActor :type "Actor Object Reference") (OtherComp :type "PrimitiveComponent Object Reference") (OtherBodyIndex :type Integer) (bFromSweep :type Boolean) (SweepResult :type "HitResult Structure (by ref)")))

(fn `CheckInventory`
  (params (Item :type String))
  (returns (PickedUp :type Boolean))
  (return false))

(fn `UserConstructionScript`)
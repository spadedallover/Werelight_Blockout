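; BP_TableRise is an animated table prop that rises up to MaxHeight while swaying and yawing, with optional counter-tilting benches.
; Two timelines drive lerped relative transforms, one for height and one for sway, with a switch mirroring the X motion.
; The construction script places the end marker and toggles bench visibility and collision.
; BeginPlay only sets timeline play rates; no visible execution path starts the timelines or reaches the random start-position node.
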(event `self.ReceiveBeginPlay`
  ;[1 1 1] Setting stuff
  (`|ExecutionSequence`
    (:`then_0`
      (`TimelineComponent.SetPlayRate` (`self.Timeline_0`) (`self.Play Rate`))
      (`TimelineComponent.SetPlayRate` (`self.Timeline_1`) (`self.Play Rate`)))))

(event `Key|E`
  (params (Key :type "Key Structure"))
  ;[1 1 1] Time Mechanic
)

(event `Key|Q`
  (params (Key :type "Key Structure"))
  ;[1 1 1] Time Mechanic
)

(fn `UserConstructionScript`
  (bind _bench1 (`self.Bench1`))
  (`SceneComponent.K2_SetRelativeLocation` (`self.TableEndPos`) (`KismetMathLibrary.MakeVector` 0.0 0.0 (+ (`self.Max Height`) 90.0)) false false)
  (`SceneComponent.SetVisibility` _bench1 (`self.Bench?`) false)
  (`SceneComponent.SetVisibility` (`self.Bench`) (`self.Bench?`) false)
  (if (`self.Bench?`)
    (`PrimitiveComponent.SetCollisionEnabled` (`self.Bench`) "QueryAndPhysics")
    (`PrimitiveComponent.SetCollisionEnabled` _bench1 "QueryAndPhysics")
    (else
      (`PrimitiveComponent.SetCollisionEnabled` _bench1 "NoCollision")
      (`PrimitiveComponent.SetCollisionEnabled` (`self.Bench`) "NoCollision"))))
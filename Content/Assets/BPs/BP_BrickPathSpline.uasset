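; BP_BrickPathSpline is a Blueprint that lays a path of brick meshes along a spline in its construction script.
; It divides the spline length by Spacing and adds a manually attached static mesh component at each step, using world-space location and rotation.
; Each brick gets a random mesh from BrickArray, and its spline yaw is multiplied, not offset, by a random factor.
; Spline mesh nodes remain in the graph but never run.
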(fn `UserConstructionScript`
  (bind _spline (`self.Spline`))
  (bind _brickarray (`self.BrickArray`))
  (for _index (range (+ (`.ReturnValue` (`KismetMathLibrary.FMod` (`SplineComponent.GetSplineLength` (`self.Spline`)) (`self.Spacing`))) 1))
    (bind _returnvalue (* _index (`self.Spacing`)))
    (bind (_returnvalue_roll _returnvalue_pitch _returnvalue_yaw) (`KismetMathLibrary.BreakRotator` (`SplineComponent.GetRotationAtDistanceAlongSpline` _spline _returnvalue "World")))
    (bind _returnvalue_2 (`AddComponent|NODE_AddStaticMeshComponent-1` :`bManualAttachment` true :`RelativeTransform` (`KismetMathLibrary.MakeTransform` (`SplineComponent.GetLocationAtDistanceAlongSpline` _spline _returnvalue "World") (`KismetMathLibrary.MakeRotator` _returnvalue_roll _returnvalue_pitch (* _returnvalue_yaw (`KismetMathLibrary.RandomFloatInRange` (`self.Min Rotation Amount`) (`self.Max Rotation Amount`)))))))
    (`StaticMeshComponent.SetStaticMesh` _returnvalue_2 (`|GetArrayItem` _brickarray (`KismetMathLibrary.RandomIntegerInRange` 0 (- (`KismetArrayLibrary.Array_Length` _brickarray) 1))))))
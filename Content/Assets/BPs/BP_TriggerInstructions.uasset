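; BP_TriggerInstructions is a trigger that shows the time-mechanic instructions on screen.
; The first overlap with its Box creates TimeMechanicInstructions_Widget, adds it to the viewport, then calls RemoveAllWidgets after a short delay, clearing every widget rather than only this one.
; DoOnce prevents repeats.
; Tick's BP_TimeMechanic check leads to no action, and CheckInventory is a stub returning false.
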(event `self.Box.OnComponentBeginOverlap`
  (params (OverlappedComponent :type "PrimitiveComponent Object Reference") (OtherActor :type "Actor Object Reference") (OtherComp :type "PrimitiveComponent Object Reference") (OtherBodyIndex :type Integer) (bFromSweep :type Boolean) (SweepResult :type "HitResult Structure (by ref)"))
  (`/Engine/EditorBlueprintResources/StandardMacros.DoOnce` false
    (:`Completed`
      (bind _returnvalue (`|CreateWidget` "/Game/Assets/BPs/TimeMechanicInstructions_Widget.TimeMechanicInstructions_Widget_C"))
      (bind _output_get (set `self.WidgetUI` _returnvalue))
      (`UserWidget.AddToViewport` _output_get 0)
      (`KismetSystemLibrary.Delay` 6.0)
      (`WidgetLayoutLibrary.RemoveAllWidgets`))))

(event `self.ReceiveTick`
  (params (DeltaSeconds :type "Float (single-precision)"))
  (bind _asbp_time_mechanic (cast `/Game/Assets/BPs/BP_TimeMechanic` (`self.NewVar_0`)))
  (if (`/Game/Assets/BPs/BP_TimeMechanic.IsTimeMoving` _asbp_time_mechanic)
    _))

(fn `CheckInventory`
  (params (Item :type String))
  (returns (PickedUp :type Boolean))
  (return false))

(fn `UserConstructionScript`)
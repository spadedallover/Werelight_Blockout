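; BP_Lights is a configurable light prop pairing a static mesh with a point light, with optional hover motion.
; The construction script applies the mesh, shadow casting, and the light's color, scaled intensity, radius and height.
; With Hover on, BeginPlay makes the mesh movable and a timeline drives its height up to HoverAmount.
; Turn_On_Lights toggles the light's visibility; CheckInventory only returns false, and random height-offset logic is unwired.
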(event `self.ReceiveBeginPlay`
  (bind _staticmesh (`self.StaticMesh`))
  (if (`self.Hover?`)
    (`SceneComponent.SetMobility` _staticmesh "Movable")
    (`SceneComponent.K2_SetRelativeLocation` _staticmesh (0.0 0.0 0.0) false false)
    (bind (_direction _newtrack_0) (`Timeline|Timeline_0`)
      (:`Update`
        (`SceneComponent.K2_SetRelativeLocation` (`self.StaticMesh`) (`KismetMathLibrary.MakeVector` 0.0 0.0 (`KismetMathLibrary.Lerp` 0.0 (`self.Hover Amount`) _newtrack_0)) false false)))))

(event `Turn_On_Lights`
  (`SceneComponent.ToggleVisibility` (`self.PointLight`) false))

(fn `CheckInventory`
  (params (Item :type String))
  (returns (PickedUp :type Boolean))
  (return false))

(fn `UserConstructionScript`
  (bind _pointlight (`self.PointLight`))
  (`|ExecutionSequence`
    (:`then_0`
      (`StaticMeshComponent.SetStaticMesh` (`self.StaticMesh`) (`self.NewMesh`))
      (`LightComponent.SetLightColor` _pointlight (`self.Light Color`) true)
      (`LightComponent.SetIntensity` _pointlight (* (`self.Light Intensity`) 100.0))
      (`LocalLightComponent.SetAttenuationRadius` _pointlight (`self.Attenuation Radius`))
      (`SceneComponent.K2_SetRelativeLocation` _pointlight (`KismetMathLibrary.MakeVector` 0.0 0.0 (`self.Light Height Offset`)) false false)
      (`PrimitiveComponent.SetCastShadow` (`self.StaticMesh`) (`self.Cast Shadow?`)))))
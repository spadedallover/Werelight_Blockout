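; BP_PottedPlant is a potted plant prop that varies its look through randomization in the Construction Script.
; It randomizes the pot's yaw and per-axis scale, keeps its mesh or swaps to PlantPotB at even odds, and picks a plant mesh from PlantArray.
; The NewPot flag sets the plant's height to suit the pot; the PlantPotB branch also feeds the plant's Z into its Y.
; Unseeded randomness re-rolls the result on each construction.
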(fn `UserConstructionScript`
  (bind _returnvalue (`KismetMathLibrary.RandomFloatInRange` 0.8 1.2))
  (bind _plantarray (`self.PlantArray`))
  (bind _plant (`self.Plant`))
  (bind (_relativelocation_x _relativelocation_y _relativelocation_z) (`KismetMathLibrary.BreakVector` (`SceneComponent.RelativeLocation` _plant)))
  ;[1 1 1] Random Rotation
  (`SceneComponent.K2_SetRelativeRotation` (`self.Pot`) (`KismetMathLibrary.MakeRotator` 0.0 0.0 (`KismetMathLibrary.RandomFloatInRange` 0.0 359.0)) false false)
  ;[1 1 1] Random Pot
  (if (`KismetMathLibrary.RandomBoolWithWeight` 0.5)
    (set `self.newPot?` false)
    (`StaticMeshComponent.SetStaticMesh` (`self.Pot`) "/Game/Assets/Rooms/Courtyard/CourtyardProps_PlantPotB.CourtyardProps_PlantPotB")
    (else
      (set `self.newPot?` true)))
  ;[1 1 1] Random Scale
  (`SceneComponent.SetRelativeScale3D` (`self.Pot`) (`KismetMathLibrary.MakeVector` _returnvalue _returnvalue _returnvalue))
  ;[1 1 1] RandomPlant
  (`StaticMeshComponent.SetStaticMesh` (`self.Plant`) (`|GetArrayItem` _plantarray (`KismetMathLibrary.RandomIntegerInRange` 0 (- (`KismetArrayLibrary.Array_Length` _plantarray) 1))))
  (if (`self.newPot?`)
    ;[1 1 1] Plant Height Adjust
    (`SceneComponent.K2_SetRelativeLocation` _plant (`KismetMathLibrary.MakeVector` _relativelocation_x _relativelocation_y 50.0) false false)
    (else
      (`SceneComponent.K2_SetRelativeLocation` _plant (`KismetMathLibrary.MakeVector` _relativelocation_x _relativelocation_z 90.0) false false))))
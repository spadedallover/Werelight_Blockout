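; BP_DiningRoomPropArray is a randomized prop actor, named for dining room dressing.
; Its construction script picks a random mesh from the Meshes array and a random material for slot 0 from the Materials array.
; It then gives the StaticMesh component a random rotation on all three axes and a modest random uniform upscale.
; The randomness is unseeded, so the look re-rolls whenever construction reruns.
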(fn `UserConstructionScript`
  (bind _returnvalue (`KismetMathLibrary.RandomFloatInRange` 0.0 360.0))
  (bind _meshes (`self.meshes`))
  (bind _staticmesh (`self.StaticMesh`))
  (bind _staticmesh_2 (`self.StaticMesh`))
  (bind _materials (`self.Materials`))
  (`StaticMeshComponent.SetStaticMesh` _staticmesh_2 (`|GetArrayItem` _meshes (`KismetMathLibrary.RandomIntegerInRange` 0 (- (`KismetArrayLibrary.Array_Length` _meshes) 1))))
  (`PrimitiveComponent.SetMaterial` _staticmesh_2 0 (`|GetArrayItem` _materials (`KismetMathLibrary.RandomIntegerInRange` 0 (- (`KismetArrayLibrary.Array_Length` _materials) 1))))
  (`SceneComponent.K2_SetRelativeRotation` _staticmesh (`KismetMathLibrary.MakeRotator` _returnvalue _returnvalue _returnvalue) false false)
  (`SceneComponent.SetRelativeScale3D` _staticmesh (`KismetMathLibrary.Conv_DoubleToVector` (`KismetMathLibrary.RandomFloatInRange` 1.0 1.5))))
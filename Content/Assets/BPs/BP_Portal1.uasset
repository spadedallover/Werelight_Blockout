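; BP_Portal1 is a portal that teleports the first-person character to a BP_Portal2 instance when it overlaps the Box.
; The destination is picked by indexing GetAllActorsOfClass with PortalNumber, and the player lands slightly above it with rotation unchanged.
; The character's Teleported flag acts as a ready gate, cleared during the jump and restored after a short delay.
; The construction script yaws PortalCapture by CameraRotation.
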(event `self.Box.OnComponentBeginOverlap`
  (params (OverlappedComponent :type "PrimitiveComponent Object Reference") (OtherActor :type "Actor Object Reference") (OtherComp :type "PrimitiveComponent Object Reference") (OtherBodyIndex :type Integer) (bFromSweep :type Boolean) (SweepResult :type "HitResult Structure (by ref)"))
  (bind _asfirst_person_character (cast `/Game/FirstPersonBP/Blueprints/FirstPersonCharacter` OtherActor))
  (set `self.FirstPerson` _asfirst_person_character)
  (if (`/Game/FirstPersonBP/Blueprints/FirstPersonCharacter.Teleported?` (`self.FirstPerson`))
    (bind _outactors (`GameplayStatics.GetAllActorsOfClass` "/Game/Assets/BPs/BP_Portal2.BP_Portal2_C"))
    (set `/Game/FirstPersonBP/Blueprints/FirstPersonCharacter.Teleported?` false (`self.FirstPerson`))
    (`self.K2_SetActorLocationAndRotation` (`self.FirstPerson`) (+ (`self.K2_GetActorLocation` (`|GetArrayItem` _outactors (`self.PortalNumber`))) (0.0 0.0 50.0)) (`self.K2_GetActorRotation` (`self.FirstPerson`)) false false)
    (`KismetSystemLibrary.Delay` 0.5)
    (set `/Game/FirstPersonBP/Blueprints/FirstPersonCharacter.Teleported?` true (`self.FirstPerson`))))

(fn `UserConstructionScript`
  (`SceneComponent.K2_SetRelativeRotation` (`self.portalCapture`) (`KismetMathLibrary.MakeRotator` 0.0 0.0 (`self.CameraRotation`)) false false))
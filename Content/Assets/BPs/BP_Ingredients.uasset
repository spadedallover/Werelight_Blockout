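; Inspectable cauldron ingredient pickup, with mesh and material set in the construction script.
; First interaction increments the player's object count, flashes an ingredient widget, freezes the player and lerps the mesh to the inspection location, where movement axes rotate it.
; Second interaction destroys the actor and unfreezes the player.
; A separate ShowSet event raises the mesh on a timeline after a random delay.
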(event `self.ReceiveBeginPlay`
  (set `self.StartWorldRotation` (`SceneComponent.K2_GetComponentRotation` (`self.StaticMesh`))))

(event `/Game/Assets/BPs/BP_LightInterface.InteractWith`
  (params (InteractWith :type "Vector Structure"))
  (`/Engine/EditorBlueprintResources/StandardMacros.FlipFlop`
    (:`A`
      (bind _asfirst_person_character (cast `/Game/FirstPersonBP/Blueprints/FirstPersonCharacter` (`GameplayStatics.GetPlayerPawn` 0)))
      (set `/Game/FirstPersonBP/Blueprints/FirstPersonCharacter.NumberofObjects` (+ (`/Game/FirstPersonBP/Blueprints/FirstPersonCharacter.NumberofObjects` _asfirst_person_character) 1) _asfirst_person_character)
      (bind _returnvalue (`|CreateWidget` "/Game/Assets/BPs/CauldronIngredients_Widget.CauldronIngredients_Widget_C"))
      (bind _output_get (set `self.ingredients_Widget` _returnvalue))
      (`UserWidget.AddToViewport` _output_get 0)
      (bind _asfirst_person_character_2 (cast `/Game/FirstPersonBP/Blueprints/FirstPersonCharacter` (`GameplayStatics.GetPlayerPawn` 0)))
      (set `/Game/FirstPersonBP/Blueprints/FirstPersonCharacter.IsPlayerFrozen` true _asfirst_person_character_2)
      (set `self.WorldLocation` (`SceneComponent.K2_GetComponentLocation` (`/Game/FirstPersonBP/Blueprints/FirstPersonCharacter.Inspection_Location` _asfirst_person_character_2)))
      (set `self.StartWorldLocation` (`SceneComponent.K2_GetComponentLocation` (`self.StaticMesh`)))
      (set `self.StartWorldRotation` (`SceneComponent.K2_GetComponentRotation` (`self.StaticMesh`)))
      (bind (_direction _newtrack_0) (`Timeline|Timeline_1` :!label _label)
        (:`Update`
          (`SceneComponent.K2_SetWorldLocation` (`self.StaticMesh`) (`KismetMathLibrary.VLerp` (`self.StartWorldLocation`) (`self.WorldLocation`) _newtrack_0) false false)
          (`SceneComponent.K2_SetWorldRotation` (`self.StaticMesh`) (`KismetMathLibrary.RLerp` (`self.StartWorldRotation`) (`self.WorldRotation`) _newtrack_0) false false)
          (`KismetSystemLibrary.Delay` 1.0)
          (`WidgetLayoutLibrary.RemoveAllWidgets`))
        (:`Finished`
          (switch `ETimelineDirection` _direction
            (:`Forward`
              (set `self.AllowRotate` true)
              (`self.EnableInput` (`GameplayStatics.GetPlayerController` 0)))))))
    (:`B`
      (`self.K2_DestroyActor`)
      (`self.DisableInput` (`GameplayStatics.GetPlayerController` 0))
      (bind _asfirst_person_character_3 (cast `/Game/FirstPersonBP/Blueprints/FirstPersonCharacter` (`GameplayStatics.GetPlayerPawn` 0)))
      (set `/Game/FirstPersonBP/Blueprints/FirstPersonCharacter.IsPlayerFrozen` false _asfirst_person_character_3)
      (set `self.AllowRotate` false)
      (set `self.WorldRotation` (`SceneComponent.K2_GetComponentRotation` (`self.StaticMesh`)))
      (goto _label :!via `Reverse`))))

(event `InputAxis|MoveForward`
  (params (AxisValue :type "Float (single-precision)"))
  (if (`self.AllowRotate`)
    (`SceneComponent.K2_AddWorldRotation` (`self.StaticMesh`) (`KismetMathLibrary.MakeRotator` 0.0 (* (`self.GetInputAxisKeyValue`) (`self.TumbleSpeed`))) false false)))

(event `InputAxis|MoveRight`
  (params (AxisValue :type "Float (single-precision)"))
  (if (`self.AllowRotate`)
    (`SceneComponent.K2_AddWorldRotation` (`self.StaticMesh`) (`KismetMathLibrary.MakeRotator` 0.0 0.0 (* (* (`self.GetInputAxisKeyValue`) (`self.TumbleSpeed`)) -1.0)) false false)))

(event `ShowSet`
  (`KismetSystemLibrary.Delay` (`KismetMathLibrary.RandomFloatInRange` (`self.MinRiseTime`) (`self.MaxRiseTime`)))
  (bind (_direction _newtrack_0) (`Timeline|Timeline_0`)
    (:`Update`
      (`SceneComponent.K2_SetRelativeLocation` (`self.StaticMesh`) (`KismetMathLibrary.VLerp` (0.0 0.0 0.0) (`self.RiseAmount`) _newtrack_0) false false))))

(fn `CheckInventory`
  (params (Item :type String))
  (returns (PickedUp :type Boolean))
  (return false))

(fn `UserConstructionScript`
  (`StaticMeshComponent.SetStaticMesh` (`self.StaticMesh`) (`self.StaticMeshChanger`))
  (`PrimitiveComponent.SetMaterial` (`self.StaticMesh`) 0 (`self.Material_Changer`)))
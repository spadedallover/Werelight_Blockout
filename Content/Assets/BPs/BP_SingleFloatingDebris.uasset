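; BP_SingleFloatingDebris is a single piece of debris that bobs and spins in place, with its mesh picked at random from an array during construction.
; BeginPlay randomizes initial pitch and roll, then starts a timeline at a random position to desynchronize instances.
; The timeline drives relative Z offset up to MaxHeight and adds rotation on selected axes each update.
; On finishing, it replays at a new random play rate.
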(event `self.ReceiveBeginPlay`
  (bind _staticmesh (`self.StaticMesh`))
  (bind _add_rotation_amount (`self.Add Rotation Amount`))
  (bind _max_set_rotation (`self.Max Set Rotation`))
  (`|ExecutionSequence`
    (:`then_0`
      (`TimelineComponent.SetPlaybackPosition` (`self.Timeline_0`) (`KismetMathLibrary.RandomFloatInRange` 0.0 2.9) false true)
      (bind (_direction _newtrack_0) (`Timeline|Timeline_0` :!label _label)
        (:`Update`
          (`SceneComponent.K2_SetRelativeLocation` _staticmesh (`KismetMathLibrary.VLerp` (0.0 0.0 0.0) (`KismetMathLibrary.MakeVector` 0.0 0.0 (`self.Max Height`)) _newtrack_0) false false)
          (`SceneComponent.K2_AddRelativeRotation` _staticmesh (`KismetMathLibrary.MakeRotator` (select `bool` (`self.X rotation`) :`true` _add_rotation_amount) (select `bool` (`self.Y rotation`) :`true` _add_rotation_amount) (select `bool` (`self.Z rotation`) :`true` _add_rotation_amount)) false false))
        (:`Finished`
          (`TimelineComponent.SetPlayRate` (`self.Timeline_0`) (`KismetMathLibrary.RandomFloatInRange` (`self.Min Playback Time`) (`self.Max Playback Time`)))
          (goto _label :!via `PlayFromStart`))))
    (:`then_1`
      (`SceneComponent.K2_SetRelativeRotation` (`self.StaticMesh`) (`KismetMathLibrary.MakeRotator` (`KismetMathLibrary.RandomFloatInRange` 0.0 _max_set_rotation) (`KismetMathLibrary.RandomFloatInRange` 0.0 _max_set_rotation)) false false))))

(fn `UserConstructionScript`
  (bind _new_mesh (`self.New Mesh`))
  (`StaticMeshComponent.SetStaticMesh` (`self.StaticMesh`) (`|GetArrayItem` _new_mesh (`KismetMathLibrary.RandomIntegerInRange` 0 (- (`KismetArrayLibrary.Array_Length` _new_mesh) 1)))))
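; Test actor for player-controlled time scrubbing of a Level Sequence inside a trigger box.
; Box overlap enables input and sets the play rate; leaving disables input and pauses.
; Holding E plays forward and Q plays in reverse, pausing on release or when pressed at the sequence limit.
; Tick also jumps the sequence to a clamped DefaultTime every frame, which BeginPlay initializes to the midpoint.
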(event `self.ReceiveTick`
  (params (DeltaSeconds :type "Float (single-precision)"))
  (bind _sequenceplayer (`LevelSequenceActor.SequencePlayer` (`self.LevelSequence`)))
  (bind _returnvalue (`KismetMathLibrary.FClamp` (`self.DefaultTime`) 0.0 (`TimeManagementBlueprintLibrary.Conv_QualifiedFrameTimeToSeconds` (`MovieSceneSequencePlayer.GetDuration` _sequenceplayer))))
  ;[1 1 1] Scrub Time
  (`MovieSceneSequencePlayer.JumpToSeconds` _sequenceplayer _returnvalue)
  (set `self.DefaultTime` _returnvalue))

(event `self.ReceiveBeginPlay`
  (set `self.DefaultTime` (/ (`TimeManagementBlueprintLibrary.Conv_QualifiedFrameTimeToSeconds` (`MovieSceneSequencePlayer.GetDuration` (`LevelSequenceActor.SequencePlayer` (`self.LevelSequence`)))) 2.0))
  (`MovieSceneSequencePlayer.Pause` (`LevelSequenceActor.SequencePlayer` (`self.LevelSequence`)) :!label _label))

(event `self.Box.OnComponentEndOverlap`
  (params (OverlappedComponent :type "PrimitiveComponent Object Reference") (OtherActor :type "Actor Object Reference") (OtherComp :type "PrimitiveComponent Object Reference") (OtherBodyIndex :type Integer))
  (`self.DisableInput` (`GameplayStatics.GetPlayerController` 0))
  (goto _label))

(event `self.Box.OnComponentBeginOverlap`
  (params (OverlappedComponent :type "PrimitiveComponent Object Reference") (OtherActor :type "Actor Object Reference") (OtherComp :type "PrimitiveComponent Object Reference") (OtherBodyIndex :type Integer) (bFromSweep :type Boolean) (SweepResult :type "HitResult Structure (by ref)"))
  (`self.EnableInput` (`GameplayStatics.GetPlayerController` 0))
  (`MovieSceneSequencePlayer.SetPlayRate` (`LevelSequenceActor.SequencePlayer` (`self.LevelSequence`)) (`self.PlayRate`)))

(event `Key|E`
  (params (Key :type "Key Structure"))
  (bind _sequenceplayer (`LevelSequenceActor.SequencePlayer` (`self.LevelSequence`)))
  (bind _sequenceplayer_2 (`LevelSequenceActor.SequencePlayer` (`self.LevelSequence`)))
  (:`Pressed`
    (if (>= (`.Value` (break `FrameNumber` (`KismetMathLibrary.BreakQualifiedFrameTime` (`MovieSceneSequencePlayer.GetCurrentTime` _sequenceplayer_2)))) (- (`.Value` (break `FrameNumber` (`KismetMathLibrary.BreakQualifiedFrameTime` (`MovieSceneSequencePlayer.GetEndTime` _sequenceplayer_2)))) 1))
      (`MovieSceneSequencePlayer.Pause` _sequenceplayer :!label _label_2)
      (else
        (`MovieSceneSequencePlayer.Play` _sequenceplayer))))
  (:`Released`
    (goto _label_2)))

(event `Key|Q`
  (params (Key :type "Key Structure"))
  (bind _sequenceplayer (`LevelSequenceActor.SequencePlayer` (`self.LevelSequence`)))
  (:`Pressed`
    (if (<= (`.Value` (break `FrameNumber` (`KismetMathLibrary.BreakQualifiedFrameTime` (`MovieSceneSequencePlayer.GetCurrentTime` _sequenceplayer)))) (`.Value` (break `FrameNumber` (`KismetMathLibrary.BreakQualifiedFrameTime` (`MovieSceneSequencePlayer.GetStartTime` _sequenceplayer)))))
      (goto _label_2)
      (else
        (`MovieSceneSequencePlayer.PlayReverse` (`LevelSequenceActor.SequencePlayer` (`self.LevelSequence`))))))
  (:`Released`
    (goto _label_2)))

(fn `UserConstructionScript`)
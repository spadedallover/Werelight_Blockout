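; BP_DiningPropsScatter is a placeable volume that scatters physics-driven dining room props when play begins.
; The construction script sizes its box component from the BoxExtent variable.
; On BeginPlay it spawns PropAmount BP_DiningRoomPropArray actors at random points inside that box.
; Each spawned prop's static mesh gets physics simulation enabled and its collision object type set to Visibility.
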(event `self.ReceiveBeginPlay`
  (bind _box (`self.Box`))
  (bind (_returnvalue_x _returnvalue_y _returnvalue_z) (`KismetMathLibrary.BreakVector` (`KismetMathLibrary.RandomPointInBoundingBox` (`SceneComponent.K2_GetComponentLocation` _box) (`BoxComponent.BoxExtent` _box))))
  (for _ (range (`self.Prop Amount`))
    (bind _returnvalue (`|SpawnActorFromClass` "/Game/Assets/BPs/BP_DiningRoomPropArray.BP_DiningRoomPropArray_C" (`KismetMathLibrary.MakeTransform` (`KismetMathLibrary.MakeVector` _returnvalue_x _returnvalue_y _returnvalue_z)) "Undefined" "OverrideRootScale" null null))
    (bind _staticmesh (`/Game/Assets/BPs/BP_DiningRoomPropArray.StaticMesh` _returnvalue))
    (`PrimitiveComponent.SetSimulatePhysics` _staticmesh true)
    (`PrimitiveComponent.SetCollisionObjectType` _staticmesh "ECC_Visibility")))

(fn `UserConstructionScript`
  (`BoxComponent.SetBoxExtent` (`self.Box`) (`self.Box Extent`) true))
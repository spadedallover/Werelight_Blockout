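; Time-rewind circle actor: an animated dial that turns backward while Q is held and forward while E is held.
; Two timelines drive the pitch of the InnerRing and Arrow, reversing or playing on key press and stopping in place on release.
; Each press also starts a looping RotateplaneSkel animation and spawns an emitter at the actor's root, which is destroyed on release.
; BeginPlay enables player input and initializes both timelines' time.
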(event `Key|Q`
  (params (Key :type "Key Structure"))
  (bind _arrow (`self.arrow`))
  (bind _inner_ring (`self.inner_ring`))
  (bind (_relativerotation_roll _relativerotation_pitch _relativerotation_yaw) (`KismetMathLibrary.BreakRotator` (`SceneComponent.RelativeRotation` _inner_ring)))
  (bind (_relativerotation_roll_2 _relativerotation_pitch_2 _relativerotation_yaw_2) (`KismetMathLibrary.BreakRotator` (`SceneComponent.RelativeRotation` _arrow)))
  ;[1 1 1] keys
  (:`Pressed`
    (`|ExecutionSequence`
      (:`then_0`
        ;[1 1 1] timelines
        (bind (_direction _newtrack_0) (`Timeline|Timeline_0` :`NewTime` (stale `SetNewTime` `New Time`) :!via `Reverse` :!label _label)
          (:`Update`
            ;[1 1 1] rotation
            (`SceneComponent.K2_SetRelativeRotation` _inner_ring (`KismetMathLibrary.MakeRotator` _relativerotation_roll (* _newtrack_0 -90.0) _relativerotation_yaw) false false))))
      (:`then_1`
        (bind (_direction_2 _newtrack_0_2) (`Timeline|arrow_timeline` :`NewTime` (stale `SetNewTime` `New Time`) :!via `Reverse` :!label _label_2)
          (:`Update`
            (`SceneComponent.K2_SetRelativeRotation` _arrow (`KismetMathLibrary.MakeRotator` _relativerotation_roll_2 (* _newtrack_0_2 -45.0) _relativerotation_yaw_2) false false))))
      (:`then_2`
        (`SkeletalMeshComponent.PlayAnimation` (`self.rotateplane_skel`) null true))
      (:`then_3`
        (bind _returnvalue (`GameplayStatics.SpawnEmitterAtLocation` null (`SceneComponent.K2_GetComponentLocation` (`self.DefaultSceneRoot`)) (struct :`Yaw` -270.0)))
        (bind _output_get (set `self.particle_reverse_var` _returnvalue)))))
  (:`Released`
    (`|ExecutionSequence`
      (:`then_0`
        (goto _label :!via `Stop`))
      (:`then_1`
        (goto _label_2 :!via `Stop`))
      (:`then_3`
        (`ActorComponent.K2_DestroyComponent` _output_get)))))

(event `Key|E`
  (params (Key :type "Key Structure"))
  ;[1 1 1] keys
  (:`Pressed`
    (`|ExecutionSequence`
      (:`then_0`
        (goto _label))
      (:`then_1`
        (goto _label_2))
      (:`then_2`
        (`SkeletalMeshComponent.PlayAnimation` (`self.rotateplane_skel`) null true))
      (:`then_3`
        (bind _returnvalue (`GameplayStatics.SpawnEmitterAtLocation` null (`SceneComponent.K2_GetComponentLocation` (`self.DefaultSceneRoot`)) (struct :`Yaw` -270.0)))
        (bind _output_get (set `self.particle_forward_var` _returnvalue)))))
  (:`Released`
    (`|ExecutionSequence`
      (:`then_0`
        (goto _label :!via `Stop`))
      (:`then_1`
        (goto _label_2 :!via `Stop`))
      (:`then_3`
        (`ActorComponent.K2_DestroyComponent` _output_get)))))

(event `SetNewTime`
  (params (`New Time` :type "Float (double-precision)" :default 1.5))
  ;[1 1 1] set new time
  (goto _label_2 :!via `SetNewTime`))

(event `self.ReceiveBeginPlay`
  (`self.EnableInput` (`GameplayStatics.GetPlayerController` 0))
  (`|ExecutionSequence`
    (:`then_0`
      (goto _label :!via `SetNewTime`))
    (:`then_1`
      (goto _label_2 :!via `SetNewTime`))))

(fn `UserConstructionScript`)